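; BP_Marin is the PowerNapper player character, which moves along world X, jumps with sound and effects, and naps while Sleep is held.
; Sleeping swaps movement settings through BPMovementSettingsComponent, blocks movement and jump input, squashes the eyes, and shows sleep VFX, plus a cloud if airborne.
; A random sleep montage restarts on blend out, and release restores the normal state.
; BeginPlay registers Marin with the HUD widget and caches the game mode.
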(event `self.ReceiveBeginPlay`
  (`parent.ReceiveBeginPlay`)
  (`|ExecutionSequence`
    (:`then_0`
      (bind _ashud_power_napper (cast `/Game/PowerNapper/UI/HUD_PowerNapper` (`PlayerController.GetHUD` (`GameplayStatics.GetPlayerController` 0))))
      (`/Game/PowerNapper/UI/Gameplay/WBP_PowerNapper.SetPlayerReference` (`/Game/PowerNapper/UI/HUD_PowerNapper.WBP_PowerNapper` _ashud_power_napper) self))
    (:`then_1`
      (bind _asgm_power_napper (cast `/Game/PowerNapper/GameFramework/Gameplay/GM_PowerNapper` (`GameplayStatics.GetGameMode`)))
      (set `self.GameMode` _asgm_power_napper))
    (:`then_2`
      (`/Game/PowerNapper/GameFramework/Player/Components/Debug/BP_MovementSettingsComponent.SetMovement` (`self.BP_MovementSettingsComponent`) (`self.NormalMovementSettings`)))))

(event `InputAction|Sleep`
  (params (Key :type "Key Structure"))
  (bind _righteye (`self.rightEye`))
  (bind _vfx_sleeping (`self.VFX_Sleeping`))
  (bind _cloud (`self.cloud`))
  (:`Pressed`
    (set `self.bIsSleeping` true)
    (`/Game/PowerNapper/GameFramework/Player/Components/Debug/BP_MovementSettingsComponent.SetMovement` (`self.BP_MovementSettingsComponent`) (`self.SleepingMovementSettings`))
    (bind _output_get (set `self.CurrentAnimation` (`KismetArrayLibrary.Array_Random` (`self.SleepingAnimations`))))
    (`|PlayMontage` (`self.Mesh`) _output_get :!label _label
      (:`then`
        (`SceneComponent.SetRelativeScale3D` _righteye (0.1 0.05 0.08))
        (`SceneComponent.SetRelativeScale3D` (`self.leftEye`) (0.1 0.05 0.08))
        (`SceneComponent.SetHiddenInGame` _vfx_sleeping false false)
        (`ActorComponent.Activate` _vfx_sleeping true)
        (if (`NavMovementComponent.IsFalling` (`self.CharacterMovement`))
          (`SceneComponent.SetHiddenInGame` _cloud false false)))
      (:`OnBlendOut`
        (goto _label))))
  (:`Released`
    (set `self.bIsSleeping` false)
    (`/Game/PowerNapper/GameFramework/Player/Components/Debug/BP_MovementSettingsComponent.SetMovement` (`self.BP_MovementSettingsComponent`) (`self.NormalMovementSettings`))
    (bind _currentanimation (`self.CurrentAnimation`)
      (:`then`
        (`self.StopAnimMontage` _currentanimation)
        (`SceneComponent.SetRelativeScale3D` _righteye (0.1 0.1 0.08))
        (`SceneComponent.SetRelativeScale3D` (`self.leftEye`) (0.1 0.1 0.08))
        (`SceneComponent.SetHiddenInGame` _vfx_sleeping true false)
        (`ActorComponent.Deactivate` _vfx_sleeping)
        (`SceneComponent.SetHiddenInGame` _cloud true false))
      (:`else`))))

(event `InputAxis|Move Forward / Backward`
  (params (AxisValue :type "Float (single-precision)"))
  (`self.AddMovementInput` (1.0 0.0 0.0) (`KismetMathLibrary.SelectFloat` 0.0 AxisValue (`self.bIsSleeping`))))

(event `InputAction|Jump`
  (params (Key :type "Key Structure"))
  (bind _returnvalue (+ (`self.K2_GetActorLocation`) (0.0 0.0 -60.0)))
  (bind _returnvalue_2 (+ (`self.K2_GetActorLocation`) (0.0 0.0 -60.0)))
  (:`Pressed`
    (if (not (`self.bIsSleeping`))
      (if (`NavMovementComponent.IsFalling` (`self.CharacterMovement`))
        (`/Engine/EditorBlueprintResources/StandardMacros.IncrementInt` (`self.JumpCount`)
          (:`  `
            _))
        (else
          (set `self.JumpCount` 0)))
      (`self.Jump`)
      (switch `int` (`self.JumpCount`)
        (:`0`
          (`GameplayStatics.PlaySoundAtLocation` "/Game/PowerNapper/Sound/Character/SC_Jump.SC_Jump" _returnvalue (struct) 0.1 1.0 0.0 null null null null)
          (`NiagaraFunctionLibrary.SpawnSystemAtLocation` null _returnvalue (struct) (0.5 0.5 0.5)))
        (:`1`
          (`GameplayStatics.PlaySoundAtLocation` "/Game/PowerNapper/Sound/Character/SC_Jump.SC_Jump" _returnvalue_2 (struct) 0.1 1.0 0.0 null null null null)
          (`NiagaraFunctionLibrary.SpawnSystemAtLocation` "/Game/PowerNapper/VFX/VFX_Jump.VFX_Jump" _returnvalue_2 (struct) (0.5 0.5 0.5))))))
  (:`Released`
    (`self.StopJumping`)))

(fn `UserConstructionScript`)