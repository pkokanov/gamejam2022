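; Camera movement component for BP_Marin that makes the spring arm smoothly follow the player, biased toward the facing direction along world Y.
; On BeginPlay it detaches the spring arm, then each tick interpolates it toward the offset target with separate speeds per axis.
; Y speed follows curves based on distance or time since a turn, slowing when stationary, while Z catches up faster during falls.
; ResetCameraPosition snaps the arm to the target.
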(event `self.ReceiveBeginPlay`
  (bind _asbp_marin (cast `/Game/PowerNapper/GameFramework/Player/BP_Marin` (`self.GetOwner`)))
  (bind _output_get (set `self.PlayerReference` _asbp_marin))
  (bind _output_get_2 (set `self.SpringArm` (`Actor.GetComponentByClass` _output_get "/Script/Engine.SpringArmComponent")))
  (`SceneComponent.K2_DetachFromComponent` _output_get_2 "KeepWorld" "KeepWorld" "KeepWorld" true))

(event `self.ReceiveTick`
  (params (DeltaSeconds :type "Float (single-precision)"))
  (bind (_returnvalue_x _returnvalue_y) (`KismetMathLibrary.BreakVector` (`SceneComponent.GetForwardVector` (`Character.CapsuleComponent` (`self.PlayerReference`)))))
  (bind _returnvalue (> _returnvalue_y 0.0))
  (set `self.DeltaTime` DeltaSeconds)
  (if (xor (`self.bLookRight`) _returnvalue)
    (set `self.bDirectionChanged` true)
    (set `self.TimeSinceDirChange` 0.0)
    (`KismetSystemLibrary.K2_SetTimer` null "ResetDirectionChanged" 0.7)
    (elif (`self.bDirectionChanged`)
      (set `self.TimeSinceDirChange` (+ (`self.TimeSinceDirChange`) (`self.DeltaTime`)))))
  (set `self.bLookRight` _returnvalue)
  (set `self.Velocity` (`Actor.GetVelocity` (`self.PlayerReference`)))
  (`SceneComponent.K2_SetWorldLocation` (`self.SpringArm`) (`KismetMathLibrary.MakeVector` (`self.XAxis`) (`self.YAxis`) (`self.ZAxis`)) false false))

(fn `ResetCameraPosition`
  (`SceneComponent.K2_SetWorldLocation` (`self.SpringArm`) (`self.Target`) false false))

(fn `ResetDirectionChanged`
  (set `self.bDirectionChanged` false))