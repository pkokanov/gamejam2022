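; Actor component that handles character death in PowerNapper, with ragdoll, sound and game mode notification.
; Die runs once, playing a fixed drop sound plus a random death sound, ragdolling the owning Character's mesh and disabling movement.
; After a short delay it destroys the character and calls CallOnPlayerDied on GM_PowerNapper.
; A separate Respawn function calls PlayerDied on the same game mode.
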(event `Die`
  (`/Engine/EditorBlueprintResources/StandardMacros.DoOnce` false
    (:`Completed`
      (bind _ascharacter (cast `Character` (`self.GetOwner`)))
      (`GameplayStatics.PlaySound2D` "/Game/PowerNapper/Sound/Character/DropDead_1.DropDead_1" 1.0 1.0 0.0 null null)
      (`GameplayStatics.PlaySound2D` (`KismetArrayLibrary.Array_Random` (`self.DeadSounds`)) 1.0 1.0 0.0 null null)
      (bind _mesh (`Character.Mesh` _ascharacter))
      (`PrimitiveComponent.SetSimulatePhysics` _mesh true)
      (`PrimitiveComponent.SetCollisionProfileName` _mesh "Ragdoll" true)
      (`CharacterMovementComponent.DisableMovement` (`Character.CharacterMovement` _ascharacter))
      (`KismetSystemLibrary.Delay` 2.0)
      (`Actor.K2_DestroyActor` _ascharacter)
      (bind _asgm_power_napper (cast `/Game/PowerNapper/GameFramework/Gameplay/GM_PowerNapper` (`GameplayStatics.GetGameMode`)))
      (`/Game/PowerNapper/GameFramework/Gameplay/GM_PowerNapper.OnPlayerDied` _asgm_power_napper))))

(fn `Respawn`
  (bind _asgm_power_napper (cast `/Game/PowerNapper/GameFramework/Gameplay/GM_PowerNapper` (`GameplayStatics.GetGameMode`)))
  (`/Game/PowerNapper/GameFramework/Gameplay/GM_PowerNapper.PlayerDied` _asgm_power_napper))