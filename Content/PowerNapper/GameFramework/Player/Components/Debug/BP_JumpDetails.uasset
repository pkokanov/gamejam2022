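; BP_JumpDetails is a debug component for BP_Marin that measures jumps and adds a WBP_JumpDetails widget to the viewport when enabled.
; A change to Falling movement mode enables apex notification and records start position and time.
; The apex handler stores the position offset and elapsed time since that start.
; While Falling, Tick draws short-lived debug spheres below the actor's origin, tracing the airborne path.
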(event `self.ReceiveBeginPlay`
  (if (`self.isEnabled`)
    (bind _asbp_marin (cast `/Game/PowerNapper/GameFramework/Player/BP_Marin` (`self.GetOwner`)))
    (set `self.PlayerReferencee` _asbp_marin)
    (bind _returnvalue (`|CreateWidget` "/Game/PowerNapper/UI/Gameplay/Debug/WBP_JumpDetails.WBP_JumpDetails_C" (`GameplayStatics.GetPlayerController` 0)))
    (`UserWidget.AddToViewport` _returnvalue 0)
    (add `Character.OnReachedJumpApex` (`self.PlayerReferencee`) (`|CreateDelegate` :!event `OnApexReached`))
    (add `Character.MovementModeChangedDelegate` (`self.PlayerReferencee`) (delegate `CustomEvent_0`))))

(event `CustomEvent_0`
  (params (Character :type "Character Object Reference") (PrevMovementMode :type "EMovementMode Enum" :default "MOVE_None") (PreviousCustomMode :type Byte))
  (if (`|EnumEquality` (`CharacterMovementComponent.MovementMode` (`Character.CharacterMovement` Character)) "MOVE_Falling")
    (`self.OnJump`)))

(event `OnApexReached`
  (if (`self.isEnabled`)
    (set `self.JumpHeight` (- (`Actor.K2_GetActorLocation` (`self.PlayerReferencee`)) (`self.StartPos`)))
    (set `self.TotalTime` (- (`KismetMathLibrary.Now`) (`self.StartTime`)))))

(event `OnJump`
  (if (`self.isEnabled`)
    (set `CharacterMovementComponent.bNotifyApex` true (`Character.CharacterMovement` (`self.PlayerReferencee`)))
    (set `self.StartPos` (`Actor.K2_GetActorLocation` (`self.PlayerReferencee`)))
    (set `self.StartTime` (`KismetMathLibrary.Now`))))

(event `self.ReceiveTick`
  (params (DeltaSeconds :type "Float (single-precision)"))
  (if (`self.isEnabled`)
    (if (`|EnumEquality` (`CharacterMovementComponent.MovementMode` (`Character.CharacterMovement` (`self.PlayerReferencee`))) "MOVE_Falling")
      (`KismetSystemLibrary.DrawDebugSphere` (- (`Actor.K2_GetActorLocation` (`self.PlayerReferencee`)) (0.0 0.0 70.0)) 5.0 1 (struct :`R` 1.0 :`A` 1.0) 5.0))))