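; Debug component that applies a movement settings struct to its owning Character, covering jump, gravity, friction, braking and air control.
; BeginPlay caches the owner's Character and CharacterMovementComponent references.
; SetMovement copies each struct field onto those references, but its only call in this graph is disconnected.
; Unwired preset structs remain in the graph, some switching values on BP_Marin's sleeping state, and Tick does nothing.
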(event `self.ReceiveBeginPlay`
  (set `self.CharacterMovementComponent` (`Actor.GetComponentByClass` (`self.GetOwner`) "/Script/Engine.CharacterMovementComponent"))
  (bind _ascharacter (cast `Character` (`self.GetOwner`)))
  (set `self.Character` _ascharacter))

(event `self.ReceiveTick`
  (params (DeltaSeconds :type "Float (single-precision)")))

(fn `SetMovement`
  (params (MovementSettings :type "/Game/PowerNapper/GameFramework/Player/SMovementSettings Structure"))
  (set `Character.JumpMaxHoldTime` MovementSettings_JumpMaxHoldTime_4_AA514D264E214EA313739180299FB27F (`self.Character`))
  (set `Character.JumpMaxCount` MovementSettings_JumpMaxCount_39_D28B66224B7B9CC9920FA39E52EAF393 (`self.Character`))
  (set `CharacterMovementComponent.GravityScale` MovementSettings_GravityScale_8_5CC850844C2F9905B8AD3DA14792D863 (`self.CharacterMovementComponent`))
  (set `CharacterMovementComponent.MaxAcceleration` MovementSettings_MaxAcceleration_10_0D97CAAD4F82C5361819C89D7AC68A8F (`self.CharacterMovementComponent`))
  (set `CharacterMovementComponent.BrakingFrictionFactor` MovementSettings_BrakingFrictionFactor_15_7D582AE141744D2E01C8E9B38A69FC8F (`self.CharacterMovementComponent`))
  (set `CharacterMovementComponent.BrakingFriction` MovementSettings_BrakingFriction_2_ADBB6ACF42473879D8524E826FE1F220 (`self.CharacterMovementComponent`))
  (set `CharacterMovementComponent.bUseSeparateBrakingFriction` MovementSettings_UseSeparateBrakingFriction_18_0EE1F8AF45724CC9FB4166AA287816D6 (`self.CharacterMovementComponent`))
  (set `CharacterMovementComponent.GroundFriction` MovementSettings_GroundFriction_20_F6C8C0684237A6938F39998E0A1E9496 (`self.CharacterMovementComponent`))
  (set `CharacterMovementComponent.BrakingDecelerationWalking` MovementSettings_BrakingDecelerationWalking_28_441235A24B5645EBC171B98734F0CCD2 (`self.CharacterMovementComponent`))
  (set `CharacterMovementComponent.JumpZVelocity` MovementSettings_JumpZVelocity_24_F0918AA2475AF82429A99F92345F040E (`self.CharacterMovementComponent`))
  (set `CharacterMovementComponent.BrakingDecelerationFalling` MovementSettings_BrakingDecelerationFalling_27_A2B383724308FCB2BA9C4B82EE6D038B (`self.CharacterMovementComponent`))
  (set `CharacterMovementComponent.AirControl` MovementSettings_AirControl_30_E4CDDB7C43150EA1263FF9ABA33D363F (`self.CharacterMovementComponent`))
  (set `CharacterMovementComponent.AirControlBoostMultiplier` MovementSettings_AirControlBoostMultiplier_33_155FB52F4DCFFB986FD67DB3A8444463 (`self.CharacterMovementComponent`))
  (set `CharacterMovementComponent.AirControlBoostVelocityThreshold` MovementSettings_AirControlBoostVelocityThreshold_35_4154308344C6D11738D374AE939F87E0 (`self.CharacterMovementComponent`))
  (set `CharacterMovementComponent.FallingLateralFriction` MovementSettings_FallingLateralFriction_37_8D0DFAB04FF946B995C3C29D74FDD279 (`self.CharacterMovementComponent`)))