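; Game mode for PowerNapper that runs the player's energy loop, main-menu camera framing, ambience and respawn.
; A looping timer drains Marin's energy, or refills it while sleeping; at zero she sleeps briefly, then wakes at full energy.
; With the world settings' main menu on, energy and normal camera wait until StartGame, which also shows the HUD.
; On death, a new Marin spawns at the saved start location after a delay and gets possessed.
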(event `StartEnergyTimer`
  (if (`self.bAllowEnergyDrain`)
    (bind _returnvalue (`KismetSystemLibrary.K2_SetTimerDelegate` (`|CreateDelegate` :!event `ModifyEnergy`) (/ 1.0 (`self.TicksPerSecond`)) true))
    (set `self.EnergyTimer` _returnvalue)))

(event `self.ReceiveBeginPlay`
  (bind _returnvalue (`GameplayStatics.GetPlayerCharacter` 0))
  (`|ExecutionSequence`
    (:`then_0`
      (set `self.PlayerData` (make `/Game/PowerNapper/GameFramework/Checkpoint/SRespawnData` (`self.GetTransform` _returnvalue)))
      (bind _asbp_marin (cast `/Game/PowerNapper/GameFramework/Player/BP_Marin` _returnvalue))
      (set `self.PlayerReference` _asbp_marin))
    (:`then_1`
      (add `self.OnPlayerDied` (`|CreateDelegate` :!event `PlayerDied`)))
    (:`then_2`
      (if (not (`APN_WorldSettings.bUseMainMenu` (`self.GetWorldSettings`)))
        (`self.StartEnergyTimer`)))
    (:`then_3`
      (if (`APN_WorldSettings.bUseMainMenu` (`self.GetWorldSettings`))
        (set `/Game/PowerNapper/GameFramework/Player/Components/Camera/BP_CameraMovementComponent.DownBias` -50.0 (`/Game/PowerNapper/GameFramework/Player/BP_Marin.BP_CameraMovementComponent` (`self.PlayerReference`)))
        (set `/Game/PowerNapper/GameFramework/Player/Components/Camera/BP_CameraMovementComponent.LeftRightBias` -50.0 (`/Game/PowerNapper/GameFramework/Player/BP_Marin.BP_CameraMovementComponent` (`self.PlayerReference`)))
        (set `self.RememberTargetArmLength` (`SpringArmComponent.TargetArmLength` (`GameJam2022Character.CameraBoom` (`self.PlayerReference`))))
        (set `SpringArmComponent.TargetArmLength` 400.0 (`GameJam2022Character.CameraBoom` (`self.PlayerReference`)))))
    (:`then_4`
      (`GameplayStatics.PlaySound2D` "/Game/PowerNapper/Sound/Level/Ambience_1.Ambience_1" 1.0 1.0 0.0 null null))))

(event `StartGame`
  (set `/Game/PowerNapper/GameFramework/Player/Components/Camera/BP_CameraMovementComponent.DownBias` (defaults `/Game/PowerNapper/GameFramework/Player/Components/Camera/BP_CameraMovementComponent` "/Game/PowerNapper/GameFramework/Player/Components/Camera/BP_CameraMovementComponent.BP_CameraMovementComponent_C") (`/Game/PowerNapper/GameFramework/Player/BP_Marin.BP_CameraMovementComponent` (`self.PlayerReference`)))
  (set `/Game/PowerNapper/GameFramework/Player/Components/Camera/BP_CameraMovementComponent.LeftRightBias` (defaults `/Game/PowerNapper/GameFramework/Player/Components/Camera/BP_CameraMovementComponent` "/Game/PowerNapper/GameFramework/Player/Components/Camera/BP_CameraMovementComponent.BP_CameraMovementComponent_C") (`/Game/PowerNapper/GameFramework/Player/BP_Marin.BP_CameraMovementComponent` (`self.PlayerReference`)))
  (set `SpringArmComponent.TargetArmLength` (`self.RememberTargetArmLength`) (`GameJam2022Character.CameraBoom` (`self.PlayerReference`)))
  (`self.StartEnergyTimer`)
  (bind _ashud_power_napper (cast `/Game/PowerNapper/UI/HUD_PowerNapper` (`PlayerController.GetHUD` (`GameplayStatics.GetPlayerController` 0))))
  (`Widget.SetVisibility` (`/Game/PowerNapper/UI/HUD_PowerNapper.WBP_PowerNapper` _ashud_power_napper) "Visible"))

(event `ModifyEnergy`
  (bind _playerreference (`self.PlayerReference`))
  (bind _playerreference_2 (`self.PlayerReference`)
    (:`then`
      (bind _output_get (set `/Game/PowerNapper/GameFramework/Player/BP_Marin.Energy` (`KismetMathLibrary.FClamp` (- (`/Game/PowerNapper/GameFramework/Player/BP_Marin.Energy` _playerreference_2) (/ (`KismetMathLibrary.SelectFloat` (* (`self.EnergyGainPerSecond`) -1.0) (`self.EnergyDrainPerSecond`) (`/Game/PowerNapper/GameFramework/Player/BP_Marin.bIsSleeping` _playerreference_2)) (`self.TicksPerSecond`))) 0.0 (`/Game/PowerNapper/GameFramework/Player/BP_Marin.MaxEnergy` (`self.PlayerReference`))) _playerreference_2))
      (if (== _output_get 0.0)
        ;[1 1 1] Option 1: You wake up after X amount of seconds
        (set `/Game/PowerNapper/GameFramework/Player/BP_Marin.bIsSleeping` true (`self.PlayerReference`))
        (`KismetSystemLibrary.K2_PauseTimerHandle` (`self.EnergyTimer`))
        (`KismetSystemLibrary.PrintString` "SLEEPING!!!" true true (struct :`R` 1.0 :`A` 1.0) 3.0)
        (`KismetSystemLibrary.Delay` 3.0)
        (`KismetSystemLibrary.K2_UnPauseTimerHandle` (`self.EnergyTimer`))
        (set `/Game/PowerNapper/GameFramework/Player/BP_Marin.Energy` (`/Game/PowerNapper/GameFramework/Player/BP_Marin.MaxEnergy` _playerreference) _playerreference)
        (set `/Game/PowerNapper/GameFramework/Player/BP_Marin.bIsSleeping` false (`self.PlayerReference`))))
    (:`else`)))

(event `PlayerDied`
  (bind _playertransform_location (`KismetMathLibrary.BreakTransform` (break `/Game/PowerNapper/GameFramework/Checkpoint/SRespawnData` (`self.PlayerData`))))
  (`KismetSystemLibrary.Delay` (`self.RespawnDelay`))
  (bind _returnvalue (`|SpawnActorFromClass` "/Game/PowerNapper/GameFramework/Player/BP_Marin.BP_Marin_C" (`KismetMathLibrary.MakeTransform` _playertransform_location) "AdjustIfPossibleButAlwaysSpawn" "OverrideRootScale" null null))
  (`Controller.Possess` (`GameplayStatics.GetPlayerController` 0) _returnvalue)
  (set `self.PlayerReference` _returnvalue))

(fn `UserConstructionScript`)