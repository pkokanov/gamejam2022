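; BP_AmbienceProfanity is a placeable trigger that plays a random ambient profanity sound when BP_Marin overlaps its box.
; The construction script uses the ProfanityType setting (window, grandma gossip or street villagers) to pick the sound pool and set a text label naming the type.
; On overlap, it plays a random sound from that pool at raised volume, unless one is already playing.
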(event `self.Box.OnComponentBeginOverlap`
  (params (OverlappedComponent :type "PrimitiveComponent Object Reference") (OtherActor :type "Actor Object Reference") (OtherComp :type "PrimitiveComponent Object Reference") (OtherBodyIndex :type Integer) (bFromSweep :type Boolean) (SweepResult :type "HitResult Structure (by ref)"))
  (cast `/Game/PowerNapper/GameFramework/Player/BP_Marin` OtherActor)
  (if (not (`AudioComponent.IsPlaying` (`self.Audio`)))
    (`AudioComponent.SetSound` (`self.Audio`) (`KismetArrayLibrary.Array_Random` (`self.SoundsToPlay`)))
    (`AudioComponent.Play` (`self.Audio`) 0.0)
    (`AudioComponent.SetVolumeMultiplier` (`self.Audio`) 2.0)))

(fn `UserConstructionScript`
  (switch `/Game/PowerNapper/GameFramework/Placeables/AmbienceProfanity/E_ProfanityType` (`self.ProfanityType`)
    (:`NewEnumerator0`
      (set `self.SoundsToPlay` (`self.ProfanitySoundsWindow`))
      (`TextRenderComponent.K2_SetText` (`self.TextRender`) "Window"))
    (:`NewEnumerator1`
      (set `self.SoundsToPlay` (`self.ProfanitySoundsGrandmaGossip`))
      (`TextRenderComponent.K2_SetText` (`self.TextRender`) "Grandma Gossip"))
    (:`NewEnumerator2`
      (set `self.SoundsToPlay` (`self.ProfanitySoundsVillagersOnTheStreet`))
      (`TextRenderComponent.K2_SetText` (`self.TextRender`) "Villagers On The Street"))))