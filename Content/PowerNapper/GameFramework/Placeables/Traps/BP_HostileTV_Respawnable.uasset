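; BP_HostileTV_Respawnable is a trap that repeatedly launches a physics TV that kills BP_Marin on contact.
; Half a second after BeginPlay it reveals the mesh, disables its box and applies a partly random force scaled by the player's forward X.
; Its first hit kills the player or plays a drop sound, then unbinds.
; Two seconds after BeginPlay it destroys itself and spawns a copy at its starting transform, looping the trap.
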(event `self.ReceiveBeginPlay`
  (set `self.NewVar_0` (`self.GetTransform`))
  (`KismetSystemLibrary.K2_SetTimerDelegate` (delegate `CustomEvent_0`) 0.5)
  (`KismetSystemLibrary.Delay` 2.0)
  (`self.K2_DestroyActor`)
  (`|SpawnActorFromClass` "BP_HostileTV_Respawnable_C" (`self.NewVar_0`) "AlwaysSpawn" "OverrideRootScale" null null))

(event `CustomEvent_0`
  (bind _asbp_marin (cast `/Game/PowerNapper/GameFramework/Player/BP_Marin` (`GameplayStatics.GetPlayerPawn` 0)))
  (`PrimitiveComponent.SetSimulatePhysics` (`self.StaticMesh`) true)
  (bind _returnvalue_x (`KismetMathLibrary.BreakVector` (`self.GetActorForwardVector` _asbp_marin)))
  (`PrimitiveComponent.AddForce` (`self.StaticMesh`) (`KismetMathLibrary.MakeVector` (* (`KismetMathLibrary.RandomFloatInRange` -30000.0 30000.0) _returnvalue_x) 11000.0 10000.0) "None" true)
  (`PrimitiveComponent.SetCollisionEnabled` (`self.Box`) "NoCollision")
  (`SceneComponent.SetHiddenInGame` (`self.StaticMesh`) false false))

(event `self.StaticMesh.OnComponentHit`
  (params (HitComponent :type "PrimitiveComponent Object Reference") (OtherActor :type "Actor Object Reference") (OtherComp :type "PrimitiveComponent Object Reference") (NormalImpulse :type "Vector Structure") (Hit :type "HitResult Structure (by ref)"))
  (bind _asbp_marin (cast `/Game/PowerNapper/GameFramework/Player/BP_Marin` OtherActor)
    (:`then`
      (`/Game/PowerNapper/GameFramework/Player/Components/BP_DeathComponent.Die` (`/Game/PowerNapper/GameFramework/Player/BP_Marin.BP_DeathComponent` _asbp_marin)))
    (:`CastFailed`
      (`GameplayStatics.PlaySoundAtLocation` "/Game/PowerNapper/Sound/Character/DropDead_1.DropDead_1" (`SceneComponent.K2_GetComponentLocation` (`self.StaticMesh`)) (struct) 2.0 1.0 0.0 null null null null)))
  (`self.SetActorTickEnabled` false)
  (clear `PrimitiveComponent.OnComponentHit` (`self.StaticMesh`))
  (`KismetSystemLibrary.Delay` 1.25))

(fn `UserConstructionScript`)