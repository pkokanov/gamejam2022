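; BP_FallingAirConditioner is a trap: an air conditioner that drops when BP_Marin enters its trigger box.
; Until its first hit, Tick rocks the mesh's pitch with a time-based sine.
; The overlap enables physics, applies a downward acceleration and disables the box.
; The first hit kills Marin or otherwise plays a drop sound, stops Tick and further hit events, then hides and disables the mesh after a delay.
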(event `self.ReceiveTick`
  (params (DeltaSeconds :type "Float (single-precision)"))
  (`SceneComponent.K2_SetWorldRotation` (`self.StaticMesh`) (`KismetMathLibrary.MakeRotator` 0.0 (- (* (`KismetMathLibrary.Sin` (`GameplayStatics.GetTimeSeconds`)) 15.0) 60.0)) false false))

(event `self.Box.OnComponentBeginOverlap`
  (params (OverlappedComponent :type "PrimitiveComponent Object Reference") (OtherActor :type "Actor Object Reference") (OtherComp :type "PrimitiveComponent Object Reference") (OtherBodyIndex :type Integer) (bFromSweep :type Boolean) (SweepResult :type "HitResult Structure (by ref)"))
  (cast `/Game/PowerNapper/GameFramework/Player/BP_Marin` OtherActor)
  (`PrimitiveComponent.SetSimulatePhysics` (`self.StaticMesh`) true)
  (`PrimitiveComponent.AddForce` (`self.StaticMesh`) (0.0 0.0 -10000.0) "None" true)
  (`PrimitiveComponent.SetCollisionEnabled` (`self.Box`) "NoCollision"))

(event `self.StaticMesh.OnComponentHit`
  (params (HitComponent :type "PrimitiveComponent Object Reference") (OtherActor :type "Actor Object Reference") (OtherComp :type "PrimitiveComponent Object Reference") (NormalImpulse :type "Vector Structure") (Hit :type "HitResult Structure (by ref)"))
  (bind _asbp_marin (cast `/Game/PowerNapper/GameFramework/Player/BP_Marin` OtherActor)
    (:`then`
      (`/Game/PowerNapper/GameFramework/Player/Components/BP_DeathComponent.Die` (`/Game/PowerNapper/GameFramework/Player/BP_Marin.BP_DeathComponent` _asbp_marin)))
    (:`CastFailed`
      (`GameplayStatics.PlaySound2D` "/Game/PowerNapper/Sound/Character/DropDead_1.DropDead_1" 1.0 1.0 0.0 null null)))
  (`self.SetActorTickEnabled` false)
  (clear `PrimitiveComponent.OnComponentHit` (`self.StaticMesh`))
  (`KismetSystemLibrary.Delay` 1.5)
  (`SceneComponent.SetHiddenInGame` (`self.StaticMesh`) true false)
  (`PrimitiveComponent.SetSimulatePhysics` (`self.StaticMesh`) false)
  (`PrimitiveComponent.SetCollisionEnabled` (`self.StaticMesh`) "NoCollision"))

(fn `UserConstructionScript`)